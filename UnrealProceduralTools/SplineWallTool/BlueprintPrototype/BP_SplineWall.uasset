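; Spline wall tool that builds walls with optional corner pieces and doors in its construction script.
; Instanced wall meshes tile each straight segment between spline points by mesh width, and instanced corners sit on the points.
; Each door entry spawns a static mesh component at a wall instance index, optionally flipped.
; Walls covered by a door, counted from one shared DoorMesh's width, are scaled to zero, keeping instance indices stable.
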(event EventBeginPlay)

(event Collision|EventActorBeginOverlap
  (params (OtherActor :type Actor%20Object%20Reference)))

(event EventTick
  (params (DeltaSeconds :type Float%20%28single-precision%29)))

(fn ConstructionScript
  (bind _spline (Variables|Default|GetSpline))
  (Components|InstancedStaticMesh|ClearInstances (Variables|Default|GetInstancedWallMesh))
  (Utilities|Array|Clear (LocalVariables|GetWallsToRemove))
  (Components|StaticMesh|SetStaticMesh (Variables|Default|GetInstancedWallMesh) (Variables|Default|GetWallMesh))
  (bind _output_get (LocalVariables|SetWallWidth (* (.y (.boxextent (StaticMesh|GetBounds (Variables|Default|GetWallMesh)))) 2.0)))
  (LocalVariables|SetNumberOfWallsForDoorSection (Math|Float|Ceil (/ (* (.y (.boxextent (StaticMesh|GetBounds (Variables|Default|GetDoorMesh)))) 2.0) _output_get)))
  (Components|StaticMesh|SetStaticMesh (Variables|Default|GetInstancedCornerMesh) (Variables|Default|GetCornerMesh))
  (Utilities|FlowControl|Sequence
    (:then_0
      ;[1 1 1] Walls
      (for _index (range 1 (- (Spline|GetNumberOfSplinePoints (Variables|Default|GetSpline)) 1))
        (LocalVariables|SetSplinePointA (Spline|GetLocationatSplinePoint _spline (- _index 1) "Local"))
        (LocalVariables|SetSplinePointB (Spline|GetLocationatSplinePoint _spline _index "Local"))
        (LocalVariables|SetNumberOfWallsThisSection (Math|Float|Floor (/ (Math|Vector|Distance(Vector) (LocalVariables|GetSplinePointA) (LocalVariables|GetSplinePointB)) (LocalVariables|GetWallWidth))))
        (LocalVariables|SetLineBA (Math|Vector|Normalize (- (LocalVariables|GetSplinePointB) (LocalVariables|GetSplinePointA))))
        (for _index_2 (range 0 (- (LocalVariables|GetNumberOfWallsThisSection) 1))
          (Components|InstancedStaticMesh|AddInstance (Variables|Default|GetInstancedWallMesh) (Math|Transform|MakeTransform (+ (LocalVariables|GetSplinePointA) (* (* _index_2 (LocalVariables|GetWallWidth)) (LocalVariables|GetLineBA))) (Math|Rotator|CombineRotators (Math|Rotator|FindLookatRotation (LocalVariables|GetSplinePointA) (LocalVariables|GetSplinePointB)) "0.000000,90.000000,0.000000")) false))))
    (:then_1
      ;[1 1 1] Corners
      (if (Variables|Default|GetUseCornerMesh)
        (if (Variables|Default|GetPlaceCornerMeshAtEnd)
          (LocalVariables|SetCornerLastIndex (- (Spline|GetNumberOfSplinePoints (Variables|Default|GetSpline)) 1))
          (else
            (LocalVariables|SetCornerLastIndex (- (Spline|GetNumberOfSplinePoints (Variables|Default|GetSpline)) 2))))
        (for _index_3 (range 0 (LocalVariables|GetCornerLastIndex))
          (Components|InstancedStaticMesh|AddInstance (Variables|Default|GetInstancedCornerMesh) (Math|Conversions|ToTransform(Vector) (Spline|GetLocationatSplinePoint (Variables|Default|GetSpline) _index_3 "Local")) false))))
    (:then_2
      ;[1 1 1] Doors
      (for _array_element (Variables|Default|GetDoors)
        (if (Class|InstancedStaticMeshComponent|IsValidInstance (Variables|Default|GetInstancedWallMesh) (.DoorPosition (Utilities|Struct|BreakBP_SplineWall_Door_Setter _array_element)))
          ;;[1 1 1] Flip the door inwards if false
          (if (.Flip (Utilities|Struct|BreakBP_SplineWall_Door_Setter _array_element))
            (LocalVariables|SetDoorScaleX (.x (.scale (.OutInstanceTransform (Components|InstancedStaticMesh|GetInstanceTransform (Variables|Default|GetInstancedWallMesh) (.DoorPosition (Utilities|Struct|BreakBP_SplineWall_Door_Setter _array_element)) false)))))
            (else
              (LocalVariables|SetDoorScaleX (* -1.0 (.x (.scale (.OutInstanceTransform (Components|InstancedStaticMesh|GetInstanceTransform (Variables|Default|GetInstancedWallMesh) (.DoorPosition (Utilities|Struct|BreakBP_SplineWall_Door_Setter _array_element)) false))))))))
          (bind _returnvalue (AddComponent|AddStaticMeshComponent false (Math|Transform|MakeTransform (.location (.OutInstanceTransform (Components|InstancedStaticMesh|GetInstanceTransform (Variables|Default|GetInstancedWallMesh) (.DoorPosition (Utilities|Struct|BreakBP_SplineWall_Door_Setter _array_element)) false))) (.rotation (.OutInstanceTransform (Components|InstancedStaticMesh|GetInstanceTransform (Variables|Default|GetInstancedWallMesh) (.DoorPosition (Utilities|Struct|BreakBP_SplineWall_Door_Setter _array_element)) false))) (Math|Vector|MakeVector (LocalVariables|GetDoorScaleX) (.y (.scale (.OutInstanceTransform (Components|InstancedStaticMesh|GetInstanceTransform (Variables|Default|GetInstancedWallMesh) (.DoorPosition (Utilities|Struct|BreakBP_SplineWall_Door_Setter _array_element)) false)))) (.z (.scale (.OutInstanceTransform (Components|InstancedStaticMesh|GetInstanceTransform (Variables|Default|GetInstancedWallMesh) (.DoorPosition (Utilities|Struct|BreakBP_SplineWall_Door_Setter _array_element)) false))))))))
          (Components|StaticMesh|SetStaticMesh _returnvalue (.DoorMesh (Utilities|Struct|BreakBP_SplineWall_Door_Setter _array_element)))
          ;;[1 1 1] We need to remove the walls that take up the same spot as the door. So we use the 'walls for door section' which tracks how many walls could fit inside a door section. Then remove the corresponding wall sections that exist in the space the door exists.
          (for _index_4 (range 0 (- (LocalVariables|GetNumberOfWallsForDoorSection) 1))
            (if (Class|InstancedStaticMeshComponent|IsValidInstance (Variables|Default|GetInstancedWallMesh) (+ (.DoorPosition (Utilities|Struct|BreakBP_SplineWall_Door_Setter _array_element)) _index_4))
              (Utilities|Array|Add (LocalVariables|GetWallsToRemove) (+ (.DoorPosition (Utilities|Struct|BreakBP_SplineWall_Door_Setter _array_element)) _index_4))))))
      (for _array_element_2 (LocalVariables|GetWallsToRemove)
        (Components|InstancedStaticMesh|UpdateInstanceTransform (Variables|Default|GetInstancedWallMesh) _array_element_2 (Math|Transform|MakeTransform "0, 0, 0" "0, 0, 0" "0.000000,0.000000,0.000000") false false true) ; Hack/Novel way to 'remove' instances without fucking up the instance IDs.
      ))))